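; Guild point actor that marks a guild's area in the world with a colored sphere and tracks player presence.
; CollisionIn overlap shows the sphere and saves the GuildID unless the player is already registered there.
; CollisionExit end-overlap hides it and resets the ID when that registered player leaves.
; BuildGuildShpere sets color and scale, then snaps the actor to static geometry via a downward line trace.
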(event OnComponentBeginOverlap(CollisionIn)
  (params (OverlappedComponent :type Primitive%20Component%20Object%20Reference) (OtherActor :type Actor%20Object%20Reference) (OtherComp :type Primitive%20Component%20Object%20Reference) (OtherBodyIndex :type Integer) (bFromSweep :type Boolean) (SweepResult :type Hit%20Result%20Structure%20%28by%20ref%29))
  (if (not (CallFunction|IsPlayerinThisGuild? OtherActor))
    (Development|SetHiddeninGame (Variables|Default|GetSphere) false false)
    (Variables|/Game/MyGame/GameMode/Buleprint/BP_SaveGame.BP_SaveGame_C|SetPlaayerLastGuildID (CallFunction|GetMySaveGame) (Variables|Default|GetGuildID))
    (Development|PrintString (Utilities|String|JoinStringArray (Utilities|Array|MakeArray "进入" "Guild" (Utilities|String|ToString(Integer) (Variables|Default|GetGuildID))) " "))))

(event OnComponentEndOverlap(CollisionExit)
  (params (OverlappedComponent :type Primitive%20Component%20Object%20Reference) (OtherActor :type Actor%20Object%20Reference) (OtherComp :type Primitive%20Component%20Object%20Reference) (OtherBodyIndex :type Integer))
  (if (CallFunction|IsPlayerinThisGuild? OtherActor)
    (Development|SetHiddeninGame (Variables|Default|GetSphere) true false)
    (Variables|/Game/MyGame/GameMode/Buleprint/BP_SaveGame.BP_SaveGame_C|SetPlaayerLastGuildID (CallFunction|GetMySaveGame) -1)
    (Development|PrintString (Utilities|String|JoinStringArray (Utilities|Array|MakeArray "离开" "Guild" (Utilities|String|ToString(Integer) (Variables|Default|GetGuildID))) " "))))

(event EventBeginPlay)

(event Collision|EventActorBeginOverlap
  (params (OtherActor :type Actor%20Object%20Reference)))

(event EventTick
  (params (DeltaSeconds :type Float%20%28single-precision%29)))

(fn ConstructionScript)

(fn GetGuildData
  (return (Default|GetGuildDatawithGuildID (CallFunction|GetMySaveGame) (Variables|Default|GetGuildID))))

(fn BuildGuildShpere
  (params (LinearColor :type Linear%20Color%20Structure%20%28by%20ref%29) (ScaleValue :type Float%20%28single-precision%29))
  (bind _returnvalue (Transformation|GetActorLocation))
  (bind _sphere (Variables|Default|GetSphere))
  (bind (_x _y) (Math|Vector|BreakVector _returnvalue))
  (Rendering|Material|SetMaterial _sphere 0 "/Game/MyGame/GameMode/Material/M_GuildSphere_Base_Inst.M_GuildSphere_Base_Inst")
  (Rendering|Material|SetVectorParameterValueonMaterials _sphere "MainColor" (Math|Conversions|ToVector(LinearColor) LinearColor))
  (Transformation|SetRelativeScale3D _sphere (Math|Vector|MakeVector ScaleValue ScaleValue ScaleValue))
  (bind (_outhit _returnvalue_2) (Collision|LineTraceForObjects _returnvalue (Math|Vector|MakeVector _x (+ _y 0.05) -3e+04) (Utilities|Array|MakeArray "ObjectTypeQuery1") false (Utilities|Array|MakeArray 0) "None"))
  (if _returnvalue_2
    (Transformation|SetActorLocation (.Location (Collision|BreakHitResult _outhit)) false false)
    (else
      (Development|PrintString "Hello"))))

(fn IsPlayerinThisGuild?
  (params (InActor :type Actor%20Object%20Reference))
  (return (and (== InActor (Game|Player|GetPlayerPawn 0)) (== (Variables|/Game/MyGame/GameMode/Buleprint/BP_SaveGame.BP_SaveGame_C|GetPlaayerLastGuildID (CallFunction|GetMySaveGame)) (Variables|Default|GetGuildID)))))