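; World map GameMode that simulates guild activity as in-game time advances, with all state held in the save game.
; NewGameTime advances the clock and resolves due actions from a queue sorted by end time, applying AP, recruits or parent-guild dominance.
; Each completion schedules that guild's next rest, recruit, patrol or war-preparation action from war state, roster, AP and hierarchy.
; Patrols score conflicts by friendship, camp, morality and randomness, but conflicts are only printed.
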(event EventBeginPlay
  (bind _asbp_game_instance (Utilities|Casting|CastToBP_GameInstance (Game|GetGameInstance)))
  (Variables|Default|SetSaveGame (Variables|/Game/MyGame/GameMode/Buleprint/BP_GameInstance.BP_GameInstance_C|GetSaveGame _asbp_game_instance)))

(event EventTick
  (params (DeltaSeconds :type Float%20%28single-precision%29)))

(event Custom|NewGameTime
  (params (InTimespan :type Timespan%20Structure))
  (bind _newparam (CallFunction|GetMySaveGame))
  (Variables|/Game/MyGame/GameMode/Buleprint/BP_SaveGame.BP_SaveGame_C|SetDateTimeInGame _newparam (+ (Variables|/Game/MyGame/GameMode/Buleprint/BP_SaveGame.BP_SaveGame_C|GetDateTimeInGame _newparam) InTimespan))
  (if (CallFunction|IsGuildActionComplate?) :!label _label
    (CallFunction|GuildActionComplate)
    (goto _label)))

(fn ConstructionScript
  (|CallParentFunction))

(fn IsGuildActionComplate?
  (bind _newparam (CallFunction|GetMySaveGame))
  (return (>= (Variables|/Game/MyGame/GameMode/Buleprint/BP_SaveGame.BP_SaveGame_C|GetDateTimeInGame _newparam) (.EndTime (Utilities|Struct|BreakS_GuildAction (Utilities|Array|Get(acopy) (Variables|/Game/MyGame/GameMode/Buleprint/BP_SaveGame.BP_SaveGame_C|GetAllGuildActionArray _newparam)))))))

(fn GuildActionComplate
  (bind _newparam (CallFunction|GetMySaveGame))
  (bind _array (Utilities|Array|MakeArray))
  (bind _allguildactionarray (Variables|/Game/MyGame/GameMode/Buleprint/BP_SaveGame.BP_SaveGame_C|GetAllGuildActionArray _newparam))
  (bind _output (Utilities|Array|Get(acopy) _allguildactionarray))
  (bind (_guildid _targetguildpointid _action _battle _starttime _endtime) (Utilities|Struct|BreakS_GuildAction _output))
  (LocalVariables|SetLocalVar_GuildID _guildid)
  (LocalVariables|SetLocalVar_TargetGuildPointID _targetguildpointid)
  (LocalVariables|SetLocalVar_GuildActionType _action)
  (Utilities|Array|RemoveItem _allguildactionarray _output)
  (Default|SetGuildIDtoinGuildArray _newparam (LocalVariables|GetLocalVar_GuildID) (LocalVariables|GetLocalVar_TargetGuildPointID) true)
  (Utilities|FlowControl|Sequence
    (:then_0
      (switch Utilities|FlowControl|Switch|SwitchonE_GuildActionType (LocalVariables|GetLocalVar_GuildActionType)
        (:NewEnumerator0
          (LocalVariables|SetLocalVar_APAdd (Math|Random|RandomIntegerinRange 1 3)))
        (:NewEnumerator2
          (for _index (range 0 (Math|Random|RandomInteger 3))
            (bind _outcharacterdata (CallFunction|RandomCharacterDataCreat))
            (Utilities|Array|Add (LocalVariables|GetLocalVar_CharacterDataArray) _outcharacterdata))
          (LocalVariables|SetLocalVar_APAdd (* (Variables|Default|GetRecruitConsume) -1)))
        (:NewEnumerator1
          (switch Utilities|FlowControl|Switch|SwitchonE_ResultOfBattle _battle
            (:NewEnumerator0
              (CallFunction|FindEnemyGuild (LocalVariables|GetLocalVar_GuildID) (LocalVariables|GetLocalVar_TargetGuildPointID)))
            (:NewEnumerator1
              _)
            (:NewEnumerator2
              _))
          ;[1 1 1] 父门派统治影响
          (if (< (.OutBattlePoint (CallFunction|GetTwoGuildBattlePoint (LocalVariables|GetLocalVar_GuildID) (.ParentGuildID (Utilities|Struct|BreakS_GuildData (Default|GetGuildDatawithGuildID (CallFunction|GetMySaveGame) (LocalVariables|GetLocalVar_GuildID)))))) -100)
            (CallFunction|SetGuildReward (.ParentGuildID (Utilities|Struct|BreakS_GuildData (Default|GetGuildDatawithGuildID (CallFunction|GetMySaveGame) (LocalVariables|GetLocalVar_GuildID)))) 0 _array -3)
            (elif (> (.OutBattlePoint (CallFunction|GetTwoGuildBattlePoint (LocalVariables|GetLocalVar_GuildID) (.ParentGuildID (Utilities|Struct|BreakS_GuildData (Default|GetGuildDatawithGuildID (CallFunction|GetMySaveGame) (LocalVariables|GetLocalVar_GuildID)))))) 100)
              (CallFunction|SetGuildReward (.ParentGuildID (Utilities|Struct|BreakS_GuildData (Default|GetGuildDatawithGuildID (CallFunction|GetMySaveGame) (LocalVariables|GetLocalVar_GuildID)))) 0 _array 3))))))
    (:then_1
      (Default|CallEDGuildActionComplate _output)
      (CallFunction|SetGuildReward (LocalVariables|GetLocalVar_GuildID) (LocalVariables|GetLocalVar_APAdd) (LocalVariables|GetLocalVar_CharacterDataArray))
      (CallFunction|NewGuildAction (LocalVariables|GetLocalVar_GuildID) _endtime))))

(fn SetGuildReward
  (params (InGuildID :type Integer) (InApAdd :type Integer) (InNewCharacterDataArray :type Array%20of%20S%20Character%20Data%20Structures) (InDominateAdd :type Integer))
  (bind _newparam (CallFunction|GetMySaveGame))
  (bind _guilddataarray (Variables|/Game/MyGame/GameMode/Buleprint/BP_SaveGame.BP_SaveGame_C|GetGuildDataArray _newparam))
  (bind _output (Utilities|Array|Get(acopy) _guilddataarray InGuildID))
  (bind (_guildtype _name _camp _moral _ap _dominate _parentguildid _characterdataarray _guildwar _guildfriendvaluearray _currguildactionarray) (Utilities|Struct|BreakS_GuildData _output))
  (Utilities|Array|AppendArray _characterdataarray InNewCharacterDataArray)
  (Utilities|Array|SetArrayElem _guilddataarray InGuildID (Utilities|Struct|MakeS_GuildData _guildtype _name _camp _moral (+ _ap InApAdd) (Math|Integer|Clamp(Integer) (+ _dominate InDominateAdd) 0 100) _parentguildid _characterdataarray _guildwar _guildfriendvaluearray _currguildactionarray))
  (return))

(fn NewGuildAction
  (params (InGuildID :type Integer) (StartTime :type Date%20Time%20Structure))
  (LocalVariables|SetLocalVar_GuildID InGuildID)
  (LocalVariables|SetLocalVar_StartTime StartTime)
  (bind _output_get (LocalVariables|SetLocalVar_GuildData (Utilities|Array|Get(acopy) (Variables|/Game/MyGame/GameMode/Buleprint/BP_SaveGame.BP_SaveGame_C|GetGuildDataArray (CallFunction|GetMySaveGame)) InGuildID)))
  (switch Utilities|FlowControl|Switch|SwitchonE_GuildWar (.GuildWar (Utilities|Struct|BreakS_GuildData _output_get))
    (:NewEnumerator0
      (Utilities|GuildActionMission (LocalVariables|GetLocalVar_GuildData)
        (:Can
          (Utilities|FindParentGuildDominate (LocalVariables|GetLocalVar_GuildID)
            (:Good
              (Utilities|GuildIsParentorNot (LocalVariables|GetLocalVar_GuildID)
                (:Yes
                  (if (!= (CallFunction|FindEnemyGuildParent (LocalVariables|GetLocalVar_GuildID)) -1)
                    _))
                (:Not
                  (CallFunction|CreatGuildActionandAddtoGuildActionArray (LocalVariables|GetLocalVar_GuildID) 0 "NewEnumerator1" (LocalVariables|GetLocalVar_StartTime) :!label _label))))
            (:Bad
              (goto _label))
            (:TooBad
              (goto _label))))
        (:Not
          (Utilities|GuildActionRecruit (LocalVariables|GetLocalVar_GuildData)
            (:Can
              (CallFunction|CreatGuildActionandAddtoGuildActionArray (LocalVariables|GetLocalVar_GuildID) 0 "NewEnumerator2" (LocalVariables|GetLocalVar_StartTime)))
            (:Not
              (CallFunction|CreatGuildActionandAddtoGuildActionArray (LocalVariables|GetLocalVar_GuildID) 0 "NewEnumerator0" (LocalVariables|GetLocalVar_StartTime)))))))
    (:NewEnumerator2
      (CallFunction|CreatGuildActionandAddtoGuildActionArray (LocalVariables|GetLocalVar_GuildID) 0 "NewEnumerator5" (LocalVariables|GetLocalVar_StartTime) :!label _label_2))
    (:NewEnumerator4
      (goto _label_2))))

(fn CreatGuildActionandAddtoGuildActionArray
  (params (InGuildID :type Integer) (InTargetGuildPointID :type Integer) (InGuildActionType :type E_GuildActionType%20Enum) (StartTime :type Date%20Time%20Structure))
  (bind _newparam (CallFunction|GetMySaveGame))
  (bind _allguildactionarray (Variables|/Game/MyGame/GameMode/Buleprint/BP_SaveGame.BP_SaveGame_C|GetAllGuildActionArray _newparam))
  (bind _guilddataarray (Variables|/Game/MyGame/GameMode/Buleprint/BP_SaveGame.BP_SaveGame_C|GetGuildDataArray _newparam))
  (bind _output (Utilities|Array|Get(acopy) _guilddataarray InGuildID))
  (bind (_guildtype _name _camp _moral _ap _dominate _parentguildid _characterdataarray _guildwar _guildfriendvaluearray _currguildactionarray) (Utilities|Struct|BreakS_GuildData _output))
  (Utilities|FlowControl|Sequence
    (:then_0
      (Default|SetGuildIDtoinGuildArray (CallFunction|GetMySaveGame) InGuildID InTargetGuildPointID false))
    (:then_1
      (bind _output_get (LocalVariables|SetLocalVar_GuildAction (Utilities|Struct|MakeS_GuildAction InGuildID InTargetGuildPointID InGuildActionType "NewEnumerator0" StartTime (+ StartTime (Math|Timespan|MakeTimespan 0 (Math|Random|RandomIntegerinRange 24 48))))))
      (Utilities|FlowControl|Sequence
        (:then_0
          (bind _output_get_2 (LocalVariables|SetNewLocalVar_0 _currguildactionarray))
          (Utilities|Array|Add _output_get_2 _output_get)
          (Utilities|Array|SetArrayElem _guilddataarray InGuildID (Utilities|Struct|MakeS_GuildData _guildtype _name _camp _moral _ap _dominate _parentguildid _characterdataarray _guildwar _guildfriendvaluearray _output_get_2) true))
        (:then_1
          (for (_array_element _array_index) _allguildactionarray
            (if (> (.EndTime (Utilities|Struct|BreakS_GuildAction _array_element)) (.EndTime (Utilities|Struct|BreakS_GuildAction _output_get)))
              (Utilities|Array|Insert _allguildactionarray _output_get _array_index)
              (Development|PrintString (Utilities|String|JoinStringArray (Utilities|Array|MakeArray "Guild" (Utilities|String|ToString(Integer) (.GuildID (Utilities|Struct|BreakS_GuildAction _output_get))) "TargetGuild" (Utilities|String|ToString(Integer) (.TargetGuildPointID (Utilities|Struct|BreakS_GuildAction _output_get))) (Utilities|String|EnumtoString (.Action (Utilities|Struct|BreakS_GuildAction _output_get))) (Utilities|String|ToString(Text) (Class|KismetTextLibrary|AsDateDateTime (.StartTime (Utilities|Struct|BreakS_GuildAction _output_get))))) " "))
              (return)))
          (Utilities|Array|Add _allguildactionarray _output_get)
          (Development|PrintString (Utilities|String|JoinStringArray (Utilities|Array|MakeArray "Guild" (Utilities|String|ToString(Integer) (.GuildID (Utilities|Struct|BreakS_GuildAction _output_get))) "TargetGuild" (Utilities|String|ToString(Integer) (.TargetGuildPointID (Utilities|Struct|BreakS_GuildAction _output_get))) (Utilities|String|EnumtoString (.Action (Utilities|Struct|BreakS_GuildAction _output_get))) (Utilities|String|ToString(Text) (Class|KismetTextLibrary|AsDateDateTime (.StartTime (Utilities|Struct|BreakS_GuildAction _output_get))))) " "))
          (return))))))

(fn FindEnemyGuildParent
  (params (InGuildID :type Integer))
  (for _array_element (Variables|/Game/MyGame/GameMode/Buleprint/BP_SaveGame.BP_SaveGame_C|GetGuildDataArray (CallFunction|GetMySaveGame))
    (if (!= (.ParentGuildID (Utilities|Struct|BreakS_GuildData (Default|GetGuildDatawithGuildID (CallFunction|GetMySaveGame) InGuildID))) (.ParentGuildID (Utilities|Struct|BreakS_GuildData _array_element)))
      (return (.ParentGuildID (Utilities|Struct|BreakS_GuildData _array_element)))))
  (return -1))

(fn FindEnemyGuild
  (params (InGuildID :type Integer) (InTargetGuildPointID :type Integer))
  (bind _newparam (CallFunction|GetMySaveGame))
  (for _array_element (Utilities|Struct|BreakS_IntArray (Utilities|Array|Get(acopy) (Variables|/Game/MyGame/GameMode/Buleprint/BP_SaveGame.BP_SaveGame_C|GetInGuildArray (CallFunction|GetMySaveGame)) InTargetGuildPointID))
    (if (== (.ParentGuildID (Utilities|Struct|BreakS_GuildData (Default|GetGuildDatawithGuildID _newparam _array_element))) (.ParentGuildID (Utilities|Struct|BreakS_GuildData (Default|GetGuildDatawithGuildID _newparam InGuildID))))
      (if (!= InGuildID _array_element)
        (Utilities|Array|Add (LocalVariables|GetGuildInParentArray) _array_element))
      (else
        (Utilities|Array|Add (LocalVariables|GetEnemyParentGuildArray) _array_element))))
  (Utilities|FlowControl|Sequence
    (:then_0
      (Utilities|FindParentGuildDominate InGuildID
        (:Good
          (LocalVariables|SetEnemyGuildArray (LocalVariables|GetEnemyParentGuildArray)))
        (:Bad
          (bind _output_get (LocalVariables|SetEnemyGuildArray (LocalVariables|GetGuildInParentArray) :!label _label))
          (Utilities|Array|AppendArray _output_get (LocalVariables|GetEnemyParentGuildArray)))
        (:TooBad
          (goto _label))))
    (:then_1
      (for _array_element_2 (LocalVariables|GetEnemyGuildArray)
        (if (< (.OutBattlePoint (CallFunction|GetTwoGuildBattlePoint InGuildID _array_element_2)) 0)
          (Development|PrintString (Utilities|String|JoinStringArray (Utilities|Array|MakeArray "Guild" (Utilities|String|ToString(Integer) InGuildID) "与" "Guild" (Utilities|String|ToString(Integer) _array_element_2) "产生冲突") " ") true true "(R=1.000000,G=0.109007,B=0.000000,A=1.000000)")
          (return)))
      (return))))

(fn GetTwoGuildBattlePoint
  (params (InGuildID :type Integer) (InTargetGuildID :type Integer))
  (bind _newparam (CallFunction|GetMySaveGame))
  (bind _outguildid (Default|GetGuildDatawithGuildID _newparam InTargetGuildID))
  (bind _outguildid_2 (Default|GetGuildDatawithGuildID _newparam InGuildID))
  (bind (_guildtype _name _camp _moral) (Utilities|Struct|BreakS_GuildData _outguildid))
  (bind (_guildtype_2 _name_2 _camp_2 _moral_2 _ap _dominate _parentguildid _characterdataarray _guildwar _guildfriendvaluearray) (Utilities|Struct|BreakS_GuildData _outguildid_2))
  (Utilities|FlowControl|Sequence
    (:then_0
      (switch Utilities|FlowControl|Switch|SwitchonE_Camp _camp_2
        (:NewEnumerator0
          (switch Utilities|FlowControl|Switch|SwitchonE_Camp _camp
            (:NewEnumerator0
              (LocalVariables|SetLocalVar_CampPoint 100 :!label _label))
            (:NewEnumerator1
              (LocalVariables|SetLocalVar_CampPoint -100 :!label _label_2))
            (:NewEnumerator2
              (LocalVariables|SetLocalVar_CampPoint 0 :!label _label_3))))
        (:NewEnumerator1
          (switch Utilities|FlowControl|Switch|SwitchonE_Camp _camp
            (:NewEnumerator0
              (goto _label_3))
            (:NewEnumerator1
              (goto _label))
            (:NewEnumerator2
              (goto _label_2))))
        (:NewEnumerator2
          (switch Utilities|FlowControl|Switch|SwitchonE_Camp _camp
            (:NewEnumerator0
              (goto _label_2))
            (:NewEnumerator1
              (goto _label_3))
            (:NewEnumerator2
              (goto _label))))))
    (:then_1
      (switch Utilities|FlowControl|Switch|SwitchonE_Moral _moral_2
        (:NewEnumerator0
          (switch Utilities|FlowControl|Switch|SwitchonE_Moral _moral
            (:NewEnumerator0
              (LocalVariables|SetLocalVar_MoralPoint 100 :!label _label_4))
            (:NewEnumerator8
              (LocalVariables|SetLocalVar_MoralPoint 0 :!label _label_5))
            (:NewEnumerator9
              (LocalVariables|SetLocalVar_MoralPoint -100 :!label _label_6))))
        (:NewEnumerator8
          (switch Utilities|FlowControl|Switch|SwitchonE_Moral _moral
            (:NewEnumerator0
              (goto _label_6))
            (:NewEnumerator8
              (goto _label_4))
            (:NewEnumerator9
              (goto _label_5))))
        (:NewEnumerator9
          (switch Utilities|FlowControl|Switch|SwitchonE_Moral _moral
            (:NewEnumerator0
              (goto _label_5))
            (:NewEnumerator8
              (goto _label_6))
            (:NewEnumerator9
              (goto _label_4))))))
    (:then_2
      (bind _output_get (LocalVariables|SetLocalVar_BattlePoint (+ (Utilities|Array|Get(acopy) _guildfriendvaluearray InTargetGuildID) (LocalVariables|GetLocalVar_CampPoint) (LocalVariables|GetLocalVar_MoralPoint) (Math|Random|RandomIntegerinRange -100 100))))
      (return _output_get InGuildID InTargetGuildID))))