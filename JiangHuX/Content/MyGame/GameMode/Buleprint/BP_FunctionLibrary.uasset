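; BP_FunctionLibrary is a Blueprint function library of shared helpers for character data, game instance access and guild coordinates.
; RandomCharacterDataCreat builds an SCharacterData with Camp and Moral each picked at random from their first two enum values.
; GetMyGameInstance casts to BP_GameInstance, and GetMySaveGame reads the SaveGame stored on it.
; GetGuildXY converts a guild ID into grid X and Y using integer division by InWeight as the row width.
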(fn RandomCharacterDataCreat
  (return (Utilities|Struct|MakeS_CharacterData "None" "None" (Utilities|Enum|ByteToEnumE_Camp (Math|Conversions|ToByte(Integer) (Math|Random|RandomInteger 2))) (Utilities|Enum|ByteToEnumE_Moral (Math|Conversions|ToByte(Integer) (Math|Random|RandomInteger 2))))))

(fn GetMyGameInstance
  (bind _asbp_game_instance (Utilities|Casting|CastToBP_GameInstance (Game|GetGameInstance)))
  (return _asbp_game_instance))

(fn GetMySaveGame
  (return (Variables|/Game/MyGame/GameMode/Buleprint/BP_GameInstance.BP_GameInstance_C|GetSaveGame (CallFunction|GetMyGameInstance))))

(fn GetGuildXY
  (params (InGuildID :type Integer) (InWeight :type Integer))
  (bind _returnvalue (/ InGuildID InWeight))
  (return (- InGuildID (* _returnvalue InWeight)) _returnvalue))