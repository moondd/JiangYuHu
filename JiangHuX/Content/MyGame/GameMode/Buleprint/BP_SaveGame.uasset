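; BP_SaveGame holds the game's guild state: guild data, guild actions and per-guild lists of guild IDs.
; NewSaveData fills it from DT_GuildData, using row names as indices and randomizing Camp, Moral and Dominate.
; One guild type also gets a self-targeted action and its own InGuildArray entry, appended without clearing earlier entries.
; Helpers read guild data, edit InGuildArray membership and apply friendship changes symmetrically to both guilds.
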(event Custom|NewSaveData
  (CallFunction|ResetGuildDataArray))

(fn ResetGuildDataArray
  (bind _outrownames (DataTable|GetDataTableRowNames "/Game/MyGame/GameMode/GameData/DT_GuildData.DT_GuildData"))
  (for _array_element _outrownames
    (bind _returnvalue (Utilities|GetDataTableRow "/Game/MyGame/GameMode/GameData/DT_GuildData.DT_GuildData" _array_element)
      (:then
        (Utilities|Array|SetArrayElem (Variables|Default|GetGuildDataArray) (Math|Conversions|ToInteger(Byte) (Utilities|String|ToString(Name) _array_element)) (Utilities|Struct|MakeS_GuildData (.GuildType (Utilities|Struct|BreakS_GuildData _returnvalue)) (.Name (Utilities|Struct|BreakS_GuildData _returnvalue)) (Utilities|Enum|ByteToEnumE_Camp (Math|Conversions|ToByte(Integer) (Math|Random|RandomIntegerinRange 0 2))) (Utilities|Enum|ByteToEnumE_Moral (Math|Conversions|ToByte(Integer) (Math|Random|RandomIntegerinRange 0 2))) (.AP (Utilities|Struct|BreakS_GuildData _returnvalue)) (Math|Random|RandomIntegerinRange 0 100) 37 (.CharacterDataArray (Utilities|Struct|BreakS_GuildData _returnvalue)) (.GuildWar (Utilities|Struct|BreakS_GuildData _returnvalue)) (.GuildFriendValueArray (Utilities|Struct|BreakS_GuildData _returnvalue)) (Utilities|Array|MakeArray)) true)
        (if (Utilities|Enum|Equal(Enum) (.GuildType (Utilities|Struct|BreakS_GuildData _returnvalue)) "NewEnumerator2")
          (Utilities|Array|Add (Variables|Default|GetAllGuildActionArray) (Utilities|Struct|MakeS_GuildAction (Math|Conversions|ToInteger(Byte) (Utilities|String|ToString(Name) _array_element)) (Math|Conversions|ToInteger(Byte) (Utilities|String|ToString(Name) _array_element))))
          (CallFunction|SetGuildIDtoinGuildArray (Math|Conversions|ToInteger(Byte) (Utilities|String|ToString(Name) _array_element)) (Math|Conversions|ToInteger(Byte) (Utilities|String|ToString(Name) _array_element)) false))))))

(fn SetGuildFriendValue
  (params (InGuildID :type Integer) (InTargetGuildID :type Integer) (InAddValue :type Integer))
  (bind _guilddataarray (Variables|Default|GetGuildDataArray))
  (bind _guilddataarray_2 (Variables|Default|GetGuildDataArray))
  (LocalVariables|SetLocalVar_GuildID InGuildID)
  (LocalVariables|SetLocalVar_TargetGuildID InTargetGuildID)
  (LocalVariables|SetLocalVar_AddValue InAddValue)
  (Utilities|Array|SetArrayElem (.GuildFriendValueArray (Utilities|Struct|BreakS_GuildData (Utilities|Array|Get(acopy) _guilddataarray_2 (LocalVariables|GetLocalVar_GuildID)))) (LocalVariables|GetLocalVar_TargetGuildID) (+ (Utilities|Array|Get(acopy) (.GuildFriendValueArray (Utilities|Struct|BreakS_GuildData (Utilities|Array|Get(acopy) _guilddataarray_2 (LocalVariables|GetLocalVar_GuildID)))) (LocalVariables|GetLocalVar_TargetGuildID)) (LocalVariables|GetLocalVar_AddValue)) true)
  (Utilities|Array|SetArrayElem _guilddataarray_2 (LocalVariables|GetLocalVar_GuildID) (Utilities|Struct|MakeS_GuildData (.GuildType (Utilities|Struct|BreakS_GuildData (Utilities|Array|Get(acopy) _guilddataarray_2 (LocalVariables|GetLocalVar_GuildID)))) (.Name (Utilities|Struct|BreakS_GuildData (Utilities|Array|Get(acopy) _guilddataarray_2 (LocalVariables|GetLocalVar_GuildID)))) (.Camp (Utilities|Struct|BreakS_GuildData (Utilities|Array|Get(acopy) _guilddataarray_2 (LocalVariables|GetLocalVar_GuildID)))) (.Moral (Utilities|Struct|BreakS_GuildData (Utilities|Array|Get(acopy) _guilddataarray_2 (LocalVariables|GetLocalVar_GuildID)))) (.AP (Utilities|Struct|BreakS_GuildData (Utilities|Array|Get(acopy) _guilddataarray_2 (LocalVariables|GetLocalVar_GuildID)))) (.Dominate (Utilities|Struct|BreakS_GuildData (Utilities|Array|Get(acopy) _guilddataarray_2 (LocalVariables|GetLocalVar_GuildID)))) (.ParentGuildID (Utilities|Struct|BreakS_GuildData (Utilities|Array|Get(acopy) _guilddataarray_2 (LocalVariables|GetLocalVar_GuildID)))) (.CharacterDataArray (Utilities|Struct|BreakS_GuildData (Utilities|Array|Get(acopy) _guilddataarray_2 (LocalVariables|GetLocalVar_GuildID)))) (.GuildWar (Utilities|Struct|BreakS_GuildData (Utilities|Array|Get(acopy) _guilddataarray_2 (LocalVariables|GetLocalVar_GuildID)))) (.GuildFriendValueArray (Utilities|Struct|BreakS_GuildData (Utilities|Array|Get(acopy) _guilddataarray_2 (LocalVariables|GetLocalVar_GuildID)))) (.CurrGuildActionArray (Utilities|Struct|BreakS_GuildData (Utilities|Array|Get(acopy) _guilddataarray_2 (LocalVariables|GetLocalVar_GuildID))))) true)
  (Utilities|Array|SetArrayElem (.GuildFriendValueArray (Utilities|Struct|BreakS_GuildData (Utilities|Array|Get(acopy) _guilddataarray (LocalVariables|GetLocalVar_TargetGuildID)))) (LocalVariables|GetLocalVar_GuildID) (+ (Utilities|Array|Get(acopy) (.GuildFriendValueArray (Utilities|Struct|BreakS_GuildData (Utilities|Array|Get(acopy) _guilddataarray (LocalVariables|GetLocalVar_TargetGuildID)))) (LocalVariables|GetLocalVar_GuildID)) (LocalVariables|GetLocalVar_AddValue)) true)
  (Utilities|Array|SetArrayElem _guilddataarray (LocalVariables|GetLocalVar_TargetGuildID) (Utilities|Struct|MakeS_GuildData (.GuildType (Utilities|Struct|BreakS_GuildData (Utilities|Array|Get(acopy) _guilddataarray (LocalVariables|GetLocalVar_TargetGuildID)))) (.Name (Utilities|Struct|BreakS_GuildData (Utilities|Array|Get(acopy) _guilddataarray (LocalVariables|GetLocalVar_TargetGuildID)))) (.Camp (Utilities|Struct|BreakS_GuildData (Utilities|Array|Get(acopy) _guilddataarray (LocalVariables|GetLocalVar_TargetGuildID)))) (.Moral (Utilities|Struct|BreakS_GuildData (Utilities|Array|Get(acopy) _guilddataarray (LocalVariables|GetLocalVar_TargetGuildID)))) (.AP (Utilities|Struct|BreakS_GuildData (Utilities|Array|Get(acopy) _guilddataarray (LocalVariables|GetLocalVar_TargetGuildID)))) (.Dominate (Utilities|Struct|BreakS_GuildData (Utilities|Array|Get(acopy) _guilddataarray (LocalVariables|GetLocalVar_TargetGuildID)))) (.ParentGuildID (Utilities|Struct|BreakS_GuildData (Utilities|Array|Get(acopy) _guilddataarray (LocalVariables|GetLocalVar_TargetGuildID)))) (.CharacterDataArray (Utilities|Struct|BreakS_GuildData (Utilities|Array|Get(acopy) _guilddataarray (LocalVariables|GetLocalVar_TargetGuildID)))) (.GuildWar (Utilities|Struct|BreakS_GuildData (Utilities|Array|Get(acopy) _guilddataarray (LocalVariables|GetLocalVar_TargetGuildID)))) (.GuildFriendValueArray (Utilities|Struct|BreakS_GuildData (Utilities|Array|Get(acopy) _guilddataarray (LocalVariables|GetLocalVar_TargetGuildID)))) (.CurrGuildActionArray (Utilities|Struct|BreakS_GuildData (Utilities|Array|Get(acopy) _guilddataarray (LocalVariables|GetLocalVar_TargetGuildID))))) true)
  (return))

(fn GetGuildFriendValue
  (params (InGuildID :type Integer) (TargetGuildID :type Integer))
  (return (Utilities|Array|Get(acopy) (.GuildFriendValueArray (Utilities|Struct|BreakS_GuildData (Utilities|Array|Get(acopy) (Variables|Default|GetGuildDataArray) InGuildID))) TargetGuildID)))

(fn GetGuildDatawithGuildID
  (params (InGuildID :type Integer))
  (return (Utilities|Array|Get(acopy) (Variables|Default|GetGuildDataArray) InGuildID)))

(fn SetGuildIDtoinGuildArray
  (params (InGuildID :type Integer) (InTargetGuildID :type Integer) (Remove :type Boolean))
  (bind _inguildarray (Variables|Default|GetInGuildArray))
  (bind _output_get (LocalVariables|SetLocalVar_Array (Utilities|Struct|BreakS_IntArray (Utilities|Array|Get(acopy) _inguildarray InTargetGuildID))))
  (if Remove
    (Utilities|Array|RemoveItem _output_get InGuildID)
    (else
      (Utilities|Array|Add _output_get InGuildID)))
  (Utilities|Array|SetArrayElem _inguildarray InTargetGuildID (Utilities|Struct|MakeS_IntArray (LocalVariables|GetLocalVar_Array)) true)
  (return))